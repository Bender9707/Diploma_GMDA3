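; Actor component that manages health (HP), shield (EP) and death for BP_BaseCharacter and BP_CustomActor owners.
; On BeginPlay it loads stats from DT_AllStats by the owner's row name, sets character walk speed and restores player HP/EP from the save unless it's a new game.
; Typed damage drains shield before HP: Piercing bypasses shield, Elemental hits shield double and HP half.
; Heal, shield and damage changes broadcast stat updates; death also broadcasts.
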(event `self.ReceiveBeginPlay`
  (`self.ConfigureStats`))

(fn `CheckEP`
  (returns (OnMax :type Boolean))
  (return (== (`self.CurrenEP`) (`.MaxEP_13_2173E6CA45A74022B13DC2A0F2464135` (break `/Game/Blueprints/Structure/STRUCT_MainStats` (`self.MainStats`))))))

(fn `CheckHP`
  (returns (OnMax :type Boolean))
  (return (== (`self.CurrenHP`) (`.MaxHP_12_56BDEBB34F2766235B7D7195B3D14660` (break `/Game/Blueprints/Structure/STRUCT_MainStats` (`self.MainStats`))))))

(fn `ConfigureMovement`
  (set `CharacterMovementComponent.MaxWalkSpeed` (`.MaxWalkSpeed_14_584A9510477E38D0AAB414A15995B752` (break `/Game/Blueprints/Structure/STRUCT_MainStats` (`self.MainStats`))) (`Character.CharacterMovement` (`self.CurrentCharacter`))))

(fn `ConfigureStats`
  (locals (L_RowName :type Name) (L_IsItCharacter :type Boolean) (L_SaveGameObj :type "/Game/Blueprints/BP_SaveGame Object Reference"))
  (bind _asbp_base_character (cast `/Game/Blueprints/Characters/BP_BaseCharacter` (`self.GetOwner`))
    (:`then`
      (set `self.CurrentCharacter` _asbp_base_character)
      (set `local.L_RowName` (`/Game/Blueprints/Characters/BP_BaseCharacter.CharacterRowName` (`self.CurrentCharacter`)))
      (set `local.L_IsItCharacter` true))
    (:`CastFailed`
      (bind _asbp_custom_actor (cast `/Game/Blueprints/BP_CustomActor` (`self.GetOwner`)))
      (set `self.CurrentCustomActor` _asbp_custom_actor)
      (set `local.L_RowName` (`/Game/Blueprints/BP_CustomActor.CustomActorRowName` (`self.CurrentCustomActor`)))
      (set `local.L_IsItCharacter` false)))
  (if (!= (`local.L_RowName`) "None")
    (bind _returnvalue (`|GetDataTableRow` "/Game/Data_Table/DT_AllStats.DT_AllStats" (`local.L_RowName`))
      (:`then`
        (set `self.MainStats` _returnvalue)
        (if (`local.L_IsItCharacter`)
          (`self.ConfigureMovement`)
          (cast `/Game/Blueprints/Characters/Player/BP_PlayerCharcter` (`self.CurrentCharacter`)
            (:`then`
              (bind _asbp_custom_game_instance (cast `/Game/Blueprints/BP_CustomGameInstance` (`GameplayStatics.GetGameInstance`))
                (:`then`
                  (if (`/Game/Blueprints/BP_CustomGameInstance.IsItNewGame` _asbp_custom_game_instance)
                    (`self.HealUp` false :!label _label)
                    (`self.ShieldUp` false)
                    (else
                      (bind _savegameobject (`/Game/Blueprints/BP_CustomGameInstance.SaveGameObject` _asbp_custom_game_instance))
                      (`/Engine/EditorBlueprintResources/StandardMacros.IsValid` _savegameobject
                        (:`Is Valid`
                          (set `local.L_SaveGameObj` _savegameobject)
                          (set `self.CurrenHP` (`/Game/Blueprints/BP_SaveGame.CurrentPlayerHP` (`local.L_SaveGameObj`)))
                          (set `self.CurrenEP` (`/Game/Blueprints/BP_SaveGame.CurrentPlayerEP` (`local.L_SaveGameObj`)))
                          (`self.OnCurrentStatsUpdated` (`self.CurrenHP`) (`self.CurrenEP`) (`self.IsDead`)))
                        (:`Is Not Valid`
                          (goto _label))))))
                (:`CastFailed`
                  (goto _label))))
            (:`CastFailed`
              (goto _label)))
          (else
            (goto _label)))
        (`self.OnConfigureStats`))
      (:`RowNotFound`
        (`KismetSystemLibrary.PrintString` "No Row Name Found" true true (struct :`R` 0.955289 :`G` 1.0 :`B` 0.0636 :`A` 1.0))))
    (else
      (`KismetSystemLibrary.PrintString` "Character has no Row Name" true true (struct :`R` 1.0 :`G` 0.155993 :`B` 0.494078 :`A` 1.0)))))

(fn `HealUp`
  (params (ToMax :type Boolean) (AddHP :type Integer))
  (locals (L_HP :type Integer))
  (if ToMax
    (set `self.CurrenHP` (`.MaxHP_12_56BDEBB34F2766235B7D7195B3D14660` (break `/Game/Blueprints/Structure/STRUCT_MainStats` (`self.MainStats`))))
    (else
      (set `local.L_HP` AddHP)
      (set `self.CurrenHP` (`KismetMathLibrary.Min` (+ (`self.CurrenHP`) (`local.L_HP`)) (`.MaxHP_12_56BDEBB34F2766235B7D7195B3D14660` (break `/Game/Blueprints/Structure/STRUCT_MainStats` (`self.MainStats`)))))))
  (`self.OnCurrentStatsUpdated` (`self.CurrenHP`) (`self.CurrenEP`) (`self.IsDead`)))

(fn `ReceveDamage`
  (params (InDamage :type Integer) (InType :type "/Game/Blueprints/Enumenators/ENUM_DamageTypes Enum" :default "NewEnumerator0"))
  (locals (L_Damage :type Integer) (L_Type :type "/Game/Blueprints/Enumenators/ENUM_DamageTypes Enum"))
  (set `local.L_Damage` InDamage)
  (set `local.L_Type` InType)
  (if (not (`self.IsDead`))
    (if (> (`self.CurrenEP`) 0)
      (switch `/Game/Blueprints/Enumenators/ENUM_DamageTypes` (`local.L_Type`)
        (:`NewEnumerator0`
          (set `self.CurrenEP` (- (`self.CurrenEP`) (`local.L_Damage`)))
          (if (not (> (`self.CurrenEP`) 0)) :!label _label
            (set `self.CurrenEP` 0))
          (set `self.IsDead` false))
        (:`NewEnumerator1`
          (set `self.CurrenEP` (- (`self.CurrenEP`) (* (`local.L_Damage`) 2)))
          (goto _label))
        (:`NewEnumerator2`
          (set `self.CurrenHP` (- (`self.CurrenHP`) (`local.L_Damage`)) :!label _label_2)
          (if (> (`self.CurrenHP`) 0) :!label _label_3
            (set `self.IsDead` false)
            (else
              (set `self.CurrenHP` 0)
              (set `self.IsDead` true)))))
      (else
        (switch `/Game/Blueprints/Enumenators/ENUM_DamageTypes` (`local.L_Type`)
          (:`NewEnumerator0`
            (goto _label_2))
          (:`NewEnumerator1`
            (set `self.CurrenHP` (- (`self.CurrenHP`) (/ (`local.L_Damage`) 2)))
            (goto _label_3))
          (:`NewEnumerator2`
            (goto _label_2)))))
    (`KismetSystemLibrary.PrintText` (`|FormatText` "{Actor} HP {hp} - EP {ep}" (`KismetTextLibrary.Conv_StringToText` (`KismetSystemLibrary.GetObjectName` (`self.GetOwner`))) (`self.CurrenHP`) (`self.CurrenEP`)) true true (select `bool` (`self.IsDead`) :`false` (struct :`R` 1.0 :`G` 1.0 :`B` 1.0 :`A` 1.0) :`true` (struct :`R` 1.0 :`A` 1.0) :!type "LinearColor Structure") 5.0)
    (`self.OnCurrentStatsUpdated` (`self.CurrenHP`) (`self.CurrenEP`) (`self.IsDead`) true)
    (if (`self.IsDead`)
      (`self.OnDied`))))

(fn `ShieldUp`
  (params (ToMax :type Boolean) (AddEP :type Integer))
  (locals (L_EP :type Integer))
  (if ToMax
    (set `self.CurrenEP` (`.MaxEP_13_2173E6CA45A74022B13DC2A0F2464135` (break `/Game/Blueprints/Structure/STRUCT_MainStats` (`self.MainStats`))))
    (else
      (set `local.L_EP` AddEP)
      (set `self.CurrenEP` (`KismetMathLibrary.Min` (+ (`self.CurrenEP`) (`local.L_EP`)) (`.MaxEP_13_2173E6CA45A74022B13DC2A0F2464135` (break `/Game/Blueprints/Structure/STRUCT_MainStats` (`self.MainStats`)))))))
  (`self.OnCurrentStatsUpdated` (`self.CurrenHP`) (`self.CurrenEP`) false (`self.IsDead`)))