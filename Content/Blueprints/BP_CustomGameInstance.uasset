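; Game instance Blueprint that manages save slots and level progression for new game, load and next-level flow.
; SaveGame creates a BP_SaveGame object if needed, fills in player HP, EP and current level, then writes the slot.
; NewGame and NextLevel save before opening a level picked from the ordered LevelPrigression array, using IsItNewGame to choose first or next.
; LoadGame reads the slot and opens its stored level.
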(fn `LoadGame`
  (params (InSlot :type String))
  (set `self.SaveGameSlot` InSlot)
  (set `self.IsItNewGame` false)
  (bind _returnvalue (`GameplayStatics.LoadGameFromSlot` (`self.SaveGameSlot`)))
  (`/Engine/EditorBlueprintResources/StandardMacros.IsValid` _returnvalue
    (:`Is Valid`
      (bind _asbp_save_game (cast `/Game/Blueprints/BP_SaveGame` _returnvalue))
      (set `self.SaveGameObject` _asbp_save_game)
      (if (!= (`/Game/Blueprints/BP_SaveGame.CurrentLevel` (`self.SaveGameObject`)) "None")
        (`GameplayStatics.OpenLevel` (`/Game/Blueprints/BP_SaveGame.CurrentLevel` (`self.SaveGameObject`)))
        (`KismetSystemLibrary.PrintString` (`KismetStringLibrary.Concat_StrStr` "LOAD GAME with level" (`KismetStringLibrary.Conv_NameToString` (`self.NextLevelName`))) true true (struct :`R` 1.0 :`G` 0.332451 :`A` 1.0) 5.0)))))

(fn `NewGame`
  (params (InSlot :type String))
  (set `self.SaveGameSlot` InSlot)
  (set `self.IsItNewGame` true)
  (bind _success (`self.SaveGame` ""))
  (if _success
    (`GameplayStatics.OpenLevel` (`/Game/Blueprints/BP_SaveGame.CurrentLevel` (`self.SaveGameObject`)))))

(fn `NextLevel`
  (bind _returnvalue (+ (`KismetArrayLibrary.Array_Find` (`self.LevelPrigression`) (`/Game/Blueprints/BP_SaveGame.CurrentLevel` (`self.SaveGameObject`))) 1))
  (set `self.IsItNewGame` false)
  (set `self.NextLevelName` (select `bool` (> _returnvalue (`KismetArrayLibrary.Array_LastIndex` (`self.LevelPrigression`))) :`false` (`|GetArrayItem` (`self.LevelPrigression`) _returnvalue)))
  (bind _success (`self.SaveGame` ""))
  (if _success
    (`GameplayStatics.OpenLevel` (`self.NextLevelName`))))

(fn `SaveGame`
  (params (SaveGameSlot :type String))
  (returns (Success :type Boolean))
  (if (`KismetStringLibrary.NotEqual_StrStr` SaveGameSlot)
    (set `self.SaveGameSlot` SaveGameSlot))
  (`self.SaveGameObject`
    (:`then`
      _)
    (:`else`
      (bind _returnvalue (`GameplayStatics.CreateSaveGameObject` "/Game/Blueprints/BP_SaveGame.BP_SaveGame_C"))
      (set `self.SaveGameObject` _returnvalue)))
  (`self.UpdateSaveGameData`)
  (bind _returnvalue_2 (`GameplayStatics.SaveGameToSlot` (`self.SaveGameObject`) (`self.SaveGameSlot`)))
  (return _returnvalue_2))

(fn `UpdateSaveGameData`
  (locals (L_Player :type "/Game/Blueprints/Characters/Player/BP_PlayerCharcter Object Reference"))
  (bind _bp_mainstatscomponent (`/Game/Blueprints/Characters/BP_BaseCharacter.BP_MainStatsComponent` (`local.L_Player`)))
  (`|ExecutionSequence`
    (:`then_0`
      (cast `/Game/Blueprints/Characters/Player/BP_PlayerCharcter` (`GameplayStatics.GetPlayerPawn` 0))
      (set `local.L_Player` null)
      (set `/Game/Blueprints/BP_SaveGame.CurrentPlayerHP` (`/Game/Blueprints/Components/BP_MainStatsComponent.CurrenHP` _bp_mainstatscomponent) (`self.SaveGameObject`))
      (set `/Game/Blueprints/BP_SaveGame.CurrentPlayerEP` (`/Game/Blueprints/Components/BP_MainStatsComponent.CurrenEP` _bp_mainstatscomponent) (`self.SaveGameObject`)))
    (:`then_1`
      (if (!= (`/Game/Blueprints/BP_SaveGame.CurrentLevel` (`self.SaveGameObject`)) "None")
        (if (`self.IsItNewGame`)
          (set `/Game/Blueprints/BP_SaveGame.CurrentLevel` (`|GetArrayItem` (`self.LevelPrigression`)) (`self.SaveGameObject`))
          (else
            (set `/Game/Blueprints/BP_SaveGame.CurrentLevel` (`self.NextLevelName`) (`self.SaveGameObject`))))
        (else
          (set `/Game/Blueprints/BP_SaveGame.CurrentLevel` (`|GetArrayItem` (`self.LevelPrigression`)) (`self.SaveGameObject`)))))))