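; Base character that owns the weapon inventory, forwards fire and reload to the current weapon, and plays hit or death sounds on stat updates.
; BeginPlay takes available weapons from the save game unless it is a new game, then equips the first.
; Weapons spawn on demand from DT_Weapons rows, attach to WeaponPoint and are cached by name, so switching toggles existing actors.
; Binds, Crouching and Interact are stubs.
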(event `self.ReceiveBeginPlay`
  (`self.Binds`)
  (`self.AvalableWeaponFromSaveGame`)
  (`self.ConfigureWeapons` 0))

(event `self.BP_MainStatsComponent.OnComponentActivated`
  (params (Component :type "ActorComponent Object Reference") (bReset :type Boolean))
  (add `/Game/Blueprints/Components/BP_MainStatsComponent.OnCurrentStatsUpdated` (`self.BP_MainStatsComponent`) (delegate `StatsUpdat`)))

(event `StatsUpdat`
  (params (CurrentHP :type Integer) (CurrentEP :type Integer) (IsDead :type Boolean) (IsItDamage :type Boolean))
  (if (not IsDead)
    (if IsItDamage
      (`AudioComponent.Play` (`self.HitSound`) 0.0))
    (else
      (`AudioComponent.Play` (`self.DeathSound`) 0.0))))

(fn `ActionMain`
  (params (`In Pressed` :type Boolean))
  (bind _currentweapon (`self.CurrentWeapon`)
    (:`then`
      (`/Game/Blueprints/Weapons/BP_BaseWeapon.ShootInputRecived` _currentweapon `In Pressed`))
    (:`else`)))

(fn `AvalableWeaponFromSaveGame`
  (bind _asbp_custom_game_instance (cast `/Game/Blueprints/BP_CustomGameInstance` (`GameplayStatics.GetGameInstance`)))
  (if (not (`/Game/Blueprints/BP_CustomGameInstance.IsItNewGame` _asbp_custom_game_instance))
    (bind _savegameobject (`/Game/Blueprints/BP_CustomGameInstance.SaveGameObject` _asbp_custom_game_instance))
    (`/Engine/EditorBlueprintResources/StandardMacros.IsValid` _savegameobject
      (:`Is Valid`
        (set `self.AvalableWeapon` (`/Game/Blueprints/BP_SaveGame.CurrentPalyerAvalableWeapon` _savegameobject))))))

(fn `Binds`)

(fn `ConfigureWeapons`
  (params (InAvalableWeaponID :type Integer))
  (locals (L_ID :type Integer) (L_Row :type "/Game/Blueprints/Structure/STRUCT_WeaponStats Structure"))
  (set `local.L_ID` InAvalableWeaponID)
  (bind _returnvalue (`|GetDataTableRow` "/Game/Data_Table/DT_Weapons.DT_Weapons" (`|GetArrayItem` (`self.AvalableWeapon`) (`local.L_ID`)))
    (:`then`
      (set `local.L_Row` _returnvalue)
      (bind _currentweapon (`self.CurrentWeapon`)
        (:`then`
          (`/Game/Blueprints/Weapons/BP_BaseWeapon.ActivateWeapon` _currentweapon false)
          (set `self.CurrentWeapon` null))
        (:`else`
          _))
      (`self.SpawnWeapon` (`|GetArrayItem` (`self.AvalableWeapon`) (`local.L_ID`)) (`.WeaponType_8_DB3A42B54A964FB5F16E11AC50428FC2` (break `/Game/Blueprints/Structure/STRUCT_WeaponStats` (`local.L_Row`)))))))

(fn `Crouching`)

(fn `GetNextWeaponName`
  (params (IsSwitchNext :type Boolean))
  (locals (L_NextWeapon :type Boolean) (L_CurrentIndex :type Integer))
  (bind (_value _returnvalue) (`BlueprintMapLibrary.Map_Find` (`self.MapOfWeapon`) (`self.CurrentWeaponName`)))
  (bind (_value_2 _returnvalue_2) (`BlueprintMapLibrary.Map_Find` (`self.MapOfWeapon`) (`self.CurrentWeaponName`)))
  (set `local.L_NextWeapon` IsSwitchNext)
  (set `local.L_CurrentIndex` (`KismetArrayLibrary.Array_Find` (`self.AvalableWeapon`) (`self.CurrentWeaponName`)))
  (if _returnvalue
    (`/Game/Blueprints/Weapons/BP_BaseWeapon.ActivateWeapon` _value false)
    (set `self.CurrentWeapon` null))
  (if (`local.L_NextWeapon`)
    (bind _result (`/Engine/EditorBlueprintResources/StandardMacros.IncrementInt` (`local.L_CurrentIndex`))
      (:`  `
        (if (<= _result (`KismetArrayLibrary.Array_LastIndex` (`self.AvalableWeapon`)))
          (set `self.CurrentWeaponName` (`|GetArrayItem` (`self.AvalableWeapon`) (`local.L_CurrentIndex`)))
          (else
            (set `self.CurrentWeaponName` (`|GetArrayItem` (`self.AvalableWeapon`)))))))
    (else
      (bind _result_2 (`/Engine/EditorBlueprintResources/StandardMacros.DecrementInt` (`local.L_CurrentIndex`))
        (:`  `
          (if (<= _result_2 0)
            (set `self.CurrentWeaponName` (`|GetArrayItem` (`self.AvalableWeapon`) (`KismetArrayLibrary.Array_LastIndex` (`self.AvalableWeapon`))))
            (else
              (set `self.CurrentWeaponName` (`|GetArrayItem` (`self.AvalableWeapon`) (`local.L_CurrentIndex`)))))))))
  (if _returnvalue_2
    (`/Game/Blueprints/Weapons/BP_BaseWeapon.ActivateWeapon` _value_2 true)
    (set `self.CurrentWeapon` _value_2)
    (`self.OnWeaponChanged`)
    (else
      (set `self.CurrentWeapon` null))))

(fn `Interact`
  (returns (Success :type Boolean))
  (return false))

(fn `ReloadWeapon`
  (`self.CurrentWeapon`
    (:`then`
      (`/Game/Blueprints/Weapons/BP_BaseWeapon.Reload` (`self.CurrentWeapon`)))
    (:`else`)))

(fn `SetWeapon`
  (bind _returnvalue (`|GetDataTableRow` "/Game/Data_Table/DT_Weapons.DT_Weapons" (`self.CurrentWeaponName`))
    (:`then`
      (`self.SpawnWeapon` (`self.CurrentWeaponName`) (`.WeaponType_8_DB3A42B54A964FB5F16E11AC50428FC2` (break `/Game/Blueprints/Structure/STRUCT_WeaponStats` _returnvalue))))))

(fn `SpawnWeapon`
  (params (InWeaponID :type Name) (InWeaponType :type "/Game/Blueprints/Enumenators/ENUM_WeaponType Enum" :default "NewEnumerator0"))
  (locals (L_WID :type Name) (L_WType :type "/Game/Blueprints/Enumenators/ENUM_WeaponType Enum"))
  (set `local.L_WID` InWeaponID)
  (set `local.L_WType` InWeaponType)
  (if (!= (`local.L_WID`) "None")
    (`self.CurrentWeapon`
      (:`then`)
      (:`else`
        (bind _returnvalue (`|SpawnActorFromClass` (select `/Game/Blueprints/Enumenators/ENUM_WeaponType` (`local.L_WType`) :`NewEnumerator0` "/Game/Blueprints/Weapons/BP_BaseWeapon_Pistol.BP_BaseWeapon_Pistol_C" :`NewEnumerator1` "/Game/Blueprints/Weapons/BP_BaseWeapon_Rifle.BP_BaseWeapon_Rifle_C" :`NewEnumerator2` "/Game/Blueprints/Weapons/BP_BaseWeapon_Shotgun.BP_BaseWeapon_Shotgun_C" :`NewEnumerator3` "/Game/Blueprints/Weapons/BP_BaseWeapon_RocketLauncher.BP_BaseWeapon_RocketLauncher_C" :!type "Actor Class Reference") (`SceneComponent.K2_GetComponentToWorld` (`self.WeaponPoint`)) "Undefined" "OverrideRootScale" self))
        (bind _asbp_base_weapon (cast `/Game/Blueprints/Weapons/BP_BaseWeapon` _returnvalue))
        (set `self.CurrentWeapon` _asbp_base_weapon)
        (`self.K2_AttachToComponent` (`self.CurrentWeapon`) (`self.WeaponPoint`) "None" "SnapToTarget" "SnapToTarget" "SnapToTarget" true)
        (bind _success (`/Game/Blueprints/Weapons/BP_BaseWeapon.WeaponConfigure` (`self.CurrentWeapon`) (`local.L_WID`)))
        (if _success
          (set `self.CurrentWeaponName` (`local.L_WID`))
          (`BlueprintMapLibrary.Map_Add` (`self.MapOfWeapon`) (`local.L_WID`) (`self.CurrentWeapon`))
          (`self.OnWeaponChanged`))))))

(fn `SwitchWeapon`
  (params (InNextWeapon :type Boolean))
  (locals (L_Next :type Boolean))
  (set `local.L_Next` InNextWeapon)
  (bind _currentweapon (`self.CurrentWeapon`)
    (:`then`
      (bind _weaponstate (`/Game/Blueprints/Weapons/BP_BaseWeapon.WeaponState` _currentweapon))
      (if (or (`|EnumInequality` _weaponstate "NewEnumerator1") (`|EnumInequality` _weaponstate "NewEnumerator3"))
        (`self.GetNextWeaponName` (`local.L_Next`) :!label _label)
        (`self.SetWeapon`)))
    (:`else`
      (goto _label))))

(fn `UpdateCustomActor`
  (params (InCustomActor :type "/Game/Blueprints/BP_CustomActor Object Reference"))
  (set `self.CustomActor` InCustomActor))

(fn `UserConstructionScript`)