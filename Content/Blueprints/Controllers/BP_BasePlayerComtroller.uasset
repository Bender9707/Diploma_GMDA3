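; Base player controller that forwards fire, reload, weapon switch, interact, crouch, jump and movement input to the possessed BP_PlayerCharcter, cached at BeginPlay.
; Most input passes through the InputAbilityCheck macro, which requires a valid, living character; Use skips the death check.
; Tick turns the character's yaw toward the cursor's trace hit, while movement follows control rotation.
; Debug prints show axis values and interaction results.
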(event `self.ReceiveBeginPlay`
  (`self.UpdateCurrentPlayerCharacter`))

(event `self.ReceiveTick`
  (params (DeltaSeconds :type "Float (single-precision)"))
  (`self.InputAbilityCheck`
    (:`True`
      (`self.UpdateRotationByMouse`)
      (`KismetSystemLibrary.PrintString` (`KismetStringLibrary.Concat_StrStr` (`KismetStringLibrary.Conv_DoubleToString` (`self.AxisMoveForwardVelue`)) " / " (`KismetStringLibrary.Conv_DoubleToString` (`self.AxisMoveRightVelue`))) true false (struct :`G` 0.66 :`B` 1.0 :`A` 1.0) 0.0))))

(event `InputAction|ActionMain`
  (params (Key :type "Key Structure"))
  ;[1 0.9333 0.9904] Shooting
  (:`Pressed`
    (`self.InputAbilityCheck`
      (:`True`
        (`/Game/Blueprints/Characters/BP_BaseCharacter.ActionMain` (`self.CurrentPlayerCharacter`) true))))
  (:`Released`
    (`self.InputAbilityCheck`
      (:`True`
        (`/Game/Blueprints/Characters/BP_BaseCharacter.ActionMain` (`self.CurrentPlayerCharacter`) false)))))

(event `InputAction|Use`
  (params (Key :type "Key Structure"))
  (:`Pressed`
    (`/Engine/EditorBlueprintResources/StandardMacros.IsValid` null
      (:`Is Valid`
        (`/Game/Blueprints/BPI_CustomInterface.Interact` (`self.CurrentPlayerCharacter`))
        (if true
          (`KismetSystemLibrary.PrintString` "Success" true true (struct :`R` 0.0115 :`G` 1.0 :`A` 1.0) 10.0)
          (else
            (`KismetSystemLibrary.PrintString` "Un Success" true true (struct :`R` 1.0 :`B` 0.047706 :`A` 1.0) 10.0))))
      (:`Is Not Valid`
        (`KismetSystemLibrary.PrintString` "Actor Not Valid!" true true (struct :`R` 1.0 :`G` 0.89218 :`A` 1.0))))))

(event `InputAxis|MoveForward`
  (params (AxisValue :type "Float (single-precision)"))
  ;[1 0.8741 0.44] Movement
  (set `self.AxisMoveForwardVelue` AxisValue)
  (`self.InputAbilityCheck`
    (:`True`
      (`Pawn.AddMovementInput` (`self.CurrentPlayerCharacter`) (`KismetMathLibrary.GetForwardVector` (`Pawn.GetControlRotation` (`self.CurrentPlayerCharacter`))) (`self.AxisMoveForwardVelue`) false))))

(event `InputAction|ReloadWeapon`
  (params (Key :type "Key Structure"))
  (:`Pressed`
    (`self.InputAbilityCheck`
      (:`True`
        (`/Game/Blueprints/Characters/BP_BaseCharacter.ReloadWeapon` (`self.CurrentPlayerCharacter`))))))

(event `InputAction|SwitchWeaponDown`
  (params (Key :type "Key Structure"))
  (:`Pressed`
    (`self.InputAbilityCheck`
      (:`True`
        (`/Game/Blueprints/Characters/BP_BaseCharacter.SwitchWeapon` (`self.CurrentPlayerCharacter`) true)))))

(event `InputAxis|MoveRight`
  (params (AxisValue :type "Float (single-precision)"))
  ;[1 0.8741 0.44] Movement
  (set `self.AxisMoveRightVelue` AxisValue)
  (`self.InputAbilityCheck`
    (:`True`
      (`Pawn.AddMovementInput` (`self.CurrentPlayerCharacter`) (`KismetMathLibrary.GetRightVector` (`Pawn.GetControlRotation` (`self.CurrentPlayerCharacter`))) (`self.AxisMoveRightVelue`) false))))

(event `InputAction|SwitchWeaponUp`
  (params (Key :type "Key Structure"))
  (:`Pressed`
    (`self.InputAbilityCheck`
      (:`True`
        (`/Game/Blueprints/Characters/BP_BaseCharacter.SwitchWeapon` (`self.CurrentPlayerCharacter`) false)))))

(event `InputAction|CrouchDown`
  (params (Key :type "Key Structure"))
  ;[0.1349 1 0] I wont only Crouch
  (:`Pressed`
    (`self.InputAbilityCheck`
      (:`True`
        (`/Game/Blueprints/Characters/BP_BaseCharacter.Crouching` (`self.CurrentPlayerCharacter`) true))))
  (:`Released`
    (`self.InputAbilityCheck`
      (:`True`
        (`/Game/Blueprints/Characters/BP_BaseCharacter.Crouching` (`self.CurrentPlayerCharacter`) false)))))

(event `InputAction|Jump`
  (params (Key :type "Key Structure"))
  (:`Pressed`
    (`self.InputAbilityCheck`
      (:`True`
        (`/Game/Blueprints/Characters/BP_BaseCharacter.Jumping` (`self.CurrentPlayerCharacter`) true))))
  (:`Released`
    (`self.InputAbilityCheck`
      (:`True`
        (`/Game/Blueprints/Characters/BP_BaseCharacter.Jumping` (`self.CurrentPlayerCharacter`) false)))))

(fn `UpdateCurrentPlayerCharacter`
  (bind _asbp_player_charcter (cast `/Game/Blueprints/Characters/Player/BP_PlayerCharcter` (`GameplayStatics.GetPlayerPawn` 0)))
  (set `self.CurrentPlayerCharacter` _asbp_player_charcter))

(fn `UpdateRotationByMouse`
  (bind (_hitresult _returnvalue) (`self.GetHitResultUnderCursorByChannel` "TraceTypeQuery1"))
  (if _returnvalue
    (set `self.New Rotation` (`KismetMathLibrary.MakeRotator` (.roll (`KismetMathLibrary.FindLookAtRotation` (`self.K2_GetActorLocation` (`self.CurrentPlayerCharacter`)) (`.Location` (`GameplayStatics.BreakHitResult` _hitresult)))) 0.0 (.yaw (`KismetMathLibrary.FindLookAtRotation` (`self.K2_GetActorLocation` (`self.CurrentPlayerCharacter`)) (`.Location` (`GameplayStatics.BreakHitResult` _hitresult))))))
    (`self.K2_SetActorRotation` (`self.CurrentPlayerCharacter`) (`self.New Rotation`) false)))

(fn `UserConstructionScript`)