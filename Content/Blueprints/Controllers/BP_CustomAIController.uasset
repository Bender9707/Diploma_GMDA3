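; AI controller for BP_BaseNPC enemies that chase and shoot the player, then drop items on death.
; Tick runs an enum state machine; pawn sensing, damage and death events switch its states.
; Chasing keeps a weapon-range band, retreating when too close (except bosses), while noises trigger a search then a timed wait.
; Waypoint patrolling via BP_AIHelper groups exists, but its call is disconnected, leaving the Patrolling state empty.
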(event `self.ReceiveBeginPlay`)

(event `self.ReceiveTick`
  (params (DeltaSeconds :type "Float (single-precision)"))
  (set `self.Delta` DeltaSeconds)
  (if (`self.CurrentCharacterConfigured`)
    (if (not (not (`/Game/Blueprints/Components/BP_MainStatsComponent.IsDead` (`/Game/Blueprints/Characters/BP_BaseCharacter.BP_MainStatsComponent` (`self.CurrentCharacter`)))))
      (set `self.AIState` "NewEnumerator5"))
    (`/Game/Blueprints/Characters/BP_BaseCharacter.ActionMain` (`self.CurrentCharacter`) false)
    (`TextRenderComponent.K2_SetText` (`/Game/Blueprints/Characters/NPC/BP_BaseNPC.TextRender` (`self.CurrentCharacter`)) (`KismetTextLibrary.Conv_StringToText` (`|GetEnumeratorNameAsString` (`self.AIState`))))
    (switch `/Game/Blueprints/Enumenators/ENUM_AIStates` (`self.AIState`)
      (:`NewEnumerator0`
        (`self.Idle`))
      (:`NewEnumerator1`
        (`self.Patrolling`))
      (:`NewEnumerator2`
        (`self.Waiting`))
      (:`NewEnumerator3`
        (`self.Chasing`))
      (:`NewEnumerator4`
        (`self.Loocking`))
      (:`NewEnumerator5`
        (`self.Death`)))
    (else
      (bind _success (`self.GetReferences`))
      (if _success
        (`self.Binds`)
        (`self.UpdateCurrentCharacter`)))))

(fn `AfterCharacterDeath`
  (bind _aftercharacterdeathhandler (`self.AfterCharacterDeathHandler`))
  (`|ExecutionSequence`
    (:`then_0`
      (if (`KismetSystemLibrary.K2_IsValidTimerHandle` _aftercharacterdeathhandler)
        (`KismetSystemLibrary.K2_ClearAndInvalidateTimerHandle` _aftercharacterdeathhandler)))
    (:`then_1`
      (`self.K2_DestroyActor` (`self.CurrentCharacter`)))))

(fn `AfterWaiting`
  (switch `/Game/Blueprints/Enumenators/ENUM_AIStates` (`self.AIState`)
    (:`NewEnumerator2`
      (`KismetSystemLibrary.K2_ClearAndInvalidateTimerHandle` (`self.AfterWaitingHandler`))
      (set `self.AIState` "NewEnumerator1"))))

(fn `Binds`
  (add `/Game/Blueprints/Characters/NPC/BP_BaseNPC.OnSeePawn` (`self.CurrentCharacter`) (`|CreateDelegate` :!event `On See Pawn`))
  (add `/Game/Blueprints/Characters/NPC/BP_BaseNPC.OnHearNoise` (`self.CurrentCharacter`) (`|CreateDelegate` :!event `OnHearNoise`))
  (add `/Game/Blueprints/Components/BP_MainStatsComponent.OnCurrentStatsUpdated` (`/Game/Blueprints/Characters/BP_BaseCharacter.BP_MainStatsComponent` (`self.CurrentCharacter`)) (`|CreateDelegate` :!event `OnDamageReceived`))
  (add `/Game/Blueprints/Components/BP_MainStatsComponent.OnDied` (`/Game/Blueprints/Characters/BP_BaseCharacter.BP_MainStatsComponent` (`self.CurrentCharacter`)) (`|CreateDelegate` :!event `OnCharacterDeath`))
  (add `/Game/Blueprints/Characters/BP_BaseCharacter.OnWeaponChanged` (`self.CurrentCharacter`) (`|CreateDelegate` :!event `OnWeaponChanged`)))

(fn `ChasePlayer`
  (if (>= (`KismetMathLibrary.VSize` (- (`self.K2_GetActorLocation` (`self.PlayerCharacter`)) (`self.Destination`))) (`self.ShootDistance`))
    (set `self.Destination` (`self.K2_GetActorLocation` (`self.PlayerCharacter`)))
    (bind _returnvalue (`self.MoveToLocation` self (`self.Destination`) (`self.ShootDistance`) true true false true null true))
    (switch `EPathFollowingRequestResult` _returnvalue
      (:`Failed`
        _)
      (:`AlreadyAtGoal`
        _))
    (set `self.AIState` "NewEnumerator4")
    (elif (> (`KismetMathLibrary.VSize` (- (`self.K2_GetActorLocation` (`self.PlayerCharacter`)) (`self.K2_GetActorLocation` (`self.CurrentCharacter`)))) (`self.StepOutDistance`))
      (`self.RotateToPlayer`)
      (`self.ShotCheck`)
      (else
        (`self.RotateToPlayer`)
        (`self.RetreatCheck`)))))

(fn `Chasing`
  (`/Game/Blueprints/Characters/BP_BaseCharacter.ActionMain` (`self.CurrentCharacter`) false)
  (`self.PlayerCharacter`
    (:`then`
      (bind _bp_mainstatscomponent (`/Game/Blueprints/Characters/BP_BaseCharacter.BP_MainStatsComponent` (`self.PlayerCharacter`))
        (:`then`
          (if (not (`/Game/Blueprints/Components/BP_MainStatsComponent.IsDead` _bp_mainstatscomponent))
            (`self.ChasePlayer`)))
        (:`else`)))
    (:`else`
      (set `self.AIState` "NewEnumerator4"))))

(fn `Death`)

(fn `FindNextPatrollLocation`
  (returns (FirstPatrolPoint :type "/Game/Blueprints/Environment/Spawners/BP_AIHelper Object Reference"))
  (locals (L_AIHelp :type "/Game/Blueprints/Environment/Spawners/BP_AIHelper Object Reference"))
  (bind _outactors (`GameplayStatics.GetAllActorsOfClass` "/Game/Blueprints/Environment/Spawners/BP_AIHelper.BP_AIHelper_C"))
  (for _array_element _outactors
    (set `local.L_AIHelp` _array_element)
    (if (== (`/Game/Blueprints/Characters/NPC/BP_BaseNPC.PatrollingGroup` (`self.CurrentCharacter`)) (`/Game/Blueprints/Environment/Spawners/BP_AIHelper.PatrollGroup` (`local.L_AIHelp`)))
      (if (== (`/Game/Blueprints/Environment/Spawners/BP_AIHelper.PatrollPointNumber` (`local.L_AIHelp`)) (`self.NextPatrollPointIndex`))
        (if (not (!= (`/Game/Blueprints/Environment/Spawners/BP_AIHelper.PatrollPointNumber` (`local.L_AIHelp`)) 0))
          (set `self.FirstPatrolPoint` (`local.L_AIHelp`)))
        (`/Engine/EditorBlueprintResources/StandardMacros.IncrementInt` (`self.NextPatrollPointIndex`)
          (:`  `
            (set `self.WalkingToPatrollPoint` true)
            (set `self.CurrentPatrolPoint` (`local.L_AIHelp`))
            (return (`self.CurrentPatrolPoint`)))))))
  (set `self.NextPatrollPointIndex` 1)
  (set `self.WalkingToPatrollPoint` true)
  (set `self.CurrentPatrolPoint` (`self.FirstPatrolPoint`))
  (return (`self.CurrentPatrolPoint`)))

(fn `GetReferences`
  (returns (Success :type Boolean))
  (bind _asbp_base_npc (cast `/Game/Blueprints/Characters/NPC/BP_BaseNPC` (`self.K2_GetPawn`))
    (:`then`
      (set `self.CurrentCharacter` _asbp_base_npc)
      (return true))
    (:`CastFailed`
      (return false))))

(fn `Idle`
  (bind _currentpatrolpoint (`self.CurrentPatrolPoint`)
    (:`then`
      (`self.InterpRotation` (`self.K2_GetActorRotation` _currentpatrolpoint)))
    (:`else`)))

(fn `InterpRotation`
  (params (InRotateTo :type "Rotator Structure"))
  (locals (L_RotateTo :type "Rotator Structure"))
  (set `local.L_RotateTo` InRotateTo)
  (`self.K2_SetActorRotation` (`self.CurrentCharacter`) (`KismetMathLibrary.RInterpTo` (`self.K2_GetActorRotation` (`self.CurrentCharacter`)) (`local.L_RotateTo`) (`self.Delta`) (`self.RotationSpeed`)) false))

(fn `Loocking`
  (set `self.PlayerCharacter` null)
  (bind _returnvalue (`self.MoveToLocation` (`self.Destination`) 150.0 true true false true null))
  (switch `EPathFollowingRequestResult` _returnvalue
    (:`AlreadyAtGoal`
      (set `self.AIState` "NewEnumerator2")
      (if (not (`KismetSystemLibrary.K2_IsValidTimerHandle` (`self.AfterCharacterDeathHandler`)))
        (bind _returnvalue_2 (`KismetSystemLibrary.K2_SetTimerDelegate` (`|CreateDelegate` :!event `AfterWaiting`) (+ (`self.WaitTime`) (`KismetMathLibrary.RandomFloatInRange` -1.0 1.0))))
        (set `self.AfterWaitingHandler` _returnvalue_2)))))

(fn `MainPatrolling`
  (if (`|EnumInequality` (`self.AIState`) "NewEnumerator2")
    (if (not (`self.WalkingToPatrollPoint`))
      (`self.FindNextPatrollLocation`)
      (set `self.Destination` (`SceneComponent.K2_GetComponentLocation` (`/Game/Blueprints/BP_CustomActor.DefaultSceneRoot` (`self.CurrentPatrolPoint`)))))
    (bind _returnvalue (`self.MoveToLocation` self (`self.Destination`) -1.0 true true true true null true))
    (switch `EPathFollowingRequestResult` _returnvalue
      (:`Failed`
        _)
      (:`AlreadyAtGoal`
        (set `self.AIState` "NewEnumerator0")
        (set `self.WalkingToPatrollPoint` false)
        (`KismetSystemLibrary.K2_SetTimerDelegate` (`|CreateDelegate` :!event `WaitingOnPatrollPoint`) (+ (`self.TimeForWaitOnPatrollPoint`) (`KismetMathLibrary.RandomFloatInRange` 0.0 5.0))))
      (:`RequestSuccessful`
        _))
    (return)))

(fn `On See Pawn`
  (params (InPawn :type "Pawn Object Reference"))
  (`self.PlayerCharacter`
    (:`then`)
    (:`else`
      (bind _asbp_player_charcter (cast `/Game/Blueprints/Characters/Player/BP_PlayerCharcter` InPawn))
      (bind _output_get (set `self.PlayerCharacter` _asbp_player_charcter))
      (set `self.Destination` (`self.K2_GetActorLocation` _output_get))
      (if (and (`|EnumInequality` (`self.AIState`) "NewEnumerator5") (`|EnumInequality` (`self.AIState`) "NewEnumerator3"))
        (set `self.AIState` "NewEnumerator3")
        (`KismetSystemLibrary.DrawDebugSphere` (`self.Destination`) 100.0 12 (struct :`R` 0.5 :`A` 1.0) 7.0 1.0)))))

(fn `OnCharacterDeath`
  (set `self.AIState` "NewEnumerator5")
  (`|ExecutionSequence`
    (:`then_0`
      (`PrimitiveComponent.SetCollisionEnabled` (`Character.CapsuleComponent` (`self.CurrentCharacter`)) "NoCollision")
      (`PrimitiveComponent.SetCollisionEnabled` (`Character.Mesh` (`self.CurrentCharacter`)) "NoCollision")
      (`SceneComponent.SetVisibility` (`/Game/Blueprints/Characters/NPC/BP_BaseNPC.LoockAtCamera` (`self.CurrentCharacter`)) false true)
      (bind _returnvalue (`KismetSystemLibrary.K2_SetTimerDelegate` (`|CreateDelegate` :!event `AfterCharacterDeath`) (`self.DeathTimer`)))
      (set `self.AfterCharacterDeathHandler` _returnvalue))
    (:`then_1`
      (for _array_element (`/Game/Blueprints/Characters/NPC/BP_BaseNPC.ItemDropClasses` (`self.CurrentCharacter`))
        (`|SpawnActorFromClass` _array_element (`KismetMathLibrary.MakeTransform` (`KismetMathLibrary.MakeVector` (.x (`self.K2_GetActorLocation` (`self.CurrentCharacter`))) (.y (`self.K2_GetActorLocation` (`self.CurrentCharacter`))) (- (.z (`self.K2_GetActorLocation` (`self.CurrentCharacter`))) (`CapsuleComponent.CapsuleHalfHeight` (`Character.CapsuleComponent` (`self.CurrentCharacter`)))))) "AdjustIfPossibleButAlwaysSpawn" "OverrideRootScale" null null)))
    (:`then_2`
      (if (`KismetSystemLibrary.IsValid` (`/Game/Blueprints/Characters/BP_BaseCharacter.CurrentWeapon` (`self.CurrentCharacter`)))
        (`self.K2_DestroyActor` (`/Game/Blueprints/Characters/BP_BaseCharacter.CurrentWeapon` (`self.CurrentCharacter`)))))))

(fn `OnDamageReceived`
  (params (InHP :type Integer) (InEP :type Integer) (IsDead :type Boolean) (IsItDamage :type Boolean))
  (if (not IsDead)
    (if IsItDamage
      (`self.UpdateCurrentPlayer`)
      (set `self.AIState` "NewEnumerator3"))
    (else
      (set `self.AIState` "NewEnumerator5"))))

(fn `OnHearNoise`
  (params (InInstigator :type "Pawn Object Reference") (InLocation :type "Vector Structure") (InVolume :type "Float (double-precision)"))
  (locals (L_Inst :type "Pawn Object Reference") (L_Loc :type "Vector Structure") (L_Vol :type "Float (double-precision)") (L_Rot :type "Rotator Structure"))
  (set `local.L_Inst` InInstigator)
  (set `local.L_Loc` InLocation)
  (set `local.L_Vol` InVolume)
  (if (> (`local.L_Vol`) 0.5)
    (if (and (`|EnumInequality` (`self.AIState`) "NewEnumerator5") (`|EnumInequality` (`self.AIState`) "NewEnumerator3"))
      (`self.K2_SetActorRotation` (`self.CurrentCharacter`) (`KismetMathLibrary.MakeRotator` (.roll (`KismetMathLibrary.FindLookAtRotation` (`self.K2_GetActorLocation` (`self.CurrentCharacter`)) (`local.L_Loc`))) 0.0 (.yaw (`KismetMathLibrary.FindLookAtRotation` (`self.K2_GetActorLocation` (`self.CurrentCharacter`)) (`local.L_Loc`)))) false)
      (set `self.Destination` (`local.L_Loc`))
      (set `self.AIState` "NewEnumerator4")
      (`KismetSystemLibrary.DrawDebugSphere` (`self.Destination`) 70.0 12 (struct :`R` 1.0 :`G` 0.332451 :`A` 1.0) 7.0 1.0))))

(fn `OnWeaponChanged`
  (`self.UpdateCurrentCharacter`))

(fn `Patrolling`)

(fn `RetreatCheck`
  (bind _capsulecomponent (`Character.CapsuleComponent` (`self.CurrentCharacter`)))
  (`/Game/Blueprints/Characters/BP_BaseCharacter.ActionMain` (`self.CurrentCharacter`) false)
  (set `self.RetreatDestination` (+ (`SceneComponent.K2_GetComponentLocation` _capsulecomponent) (* (`KismetMathLibrary.GetForwardVector` (`SceneComponent.K2_GetComponentRotation` _capsulecomponent)) (* (`self.StepOutDistance`) -1.0))))
  (`self.MoveToLocation` self (`self.RetreatDestination`) -1.0 true true false true null true))

(fn `RotateToPlayer`
  (`self.K2_SetActorRotation` (`self.CurrentCharacter`) (`KismetMathLibrary.MakeRotator` (.roll (`KismetMathLibrary.FindLookAtRotation` (`self.K2_GetActorLocation` (`self.CurrentCharacter`)) (`self.K2_GetActorLocation` (`self.PlayerCharacter`)))) 0.0 (.yaw (`KismetMathLibrary.FindLookAtRotation` (`self.K2_GetActorLocation` (`self.CurrentCharacter`)) (`self.K2_GetActorLocation` (`self.PlayerCharacter`))))) false))

(fn `ShotCheck`
  (bind _currentweapon (`/Game/Blueprints/Characters/BP_BaseCharacter.CurrentWeapon` (`self.CurrentCharacter`)))
  (switch `/Game/Blueprints/Enumenators/ENUM_WeaponState` (`/Game/Blueprints/Weapons/BP_BaseWeapon.WeaponState` (`/Game/Blueprints/Characters/BP_BaseCharacter.CurrentWeapon` (`self.CurrentCharacter`)))
    (:`NewEnumerator0`
      (`/Game/Blueprints/Characters/BP_BaseCharacter.ActionMain` (`self.CurrentCharacter`) true))
    (:`NewEnumerator2`
      (`/Game/Blueprints/Characters/BP_BaseCharacter.ActionMain` (`self.CurrentCharacter`) false :!label _label)
      (set `/Game/Blueprints/Weapons/BP_BaseWeapon.AmmoCurrent` (`/Game/Blueprints/Weapons/BP_BaseWeapon.AmmoMax` _currentweapon) _currentweapon)
      (`/Game/Blueprints/Weapons/BP_BaseWeapon.Reload` (`/Game/Blueprints/Characters/BP_BaseCharacter.CurrentWeapon` (`self.CurrentCharacter`))))
    (:`NewEnumerator4`
      (goto _label))))

(fn `UpdateCurrentCharacter`
  (`self.CurrentCharacter`
    (:`then`
      _)
    (:`else`
      (bind _asbp_base_npc (cast `/Game/Blueprints/Characters/NPC/BP_BaseNPC` (`self.K2_GetPawn`)))
      (set `self.CurrentCharacter` _asbp_base_npc)))
  (`|ExecutionSequence`
    (:`then_0`
      (bind _currentweapon (`/Game/Blueprints/Characters/BP_BaseCharacter.CurrentWeapon` (`self.CurrentCharacter`))
        (:`then`
          (set `self.ShootDistance` (`/Game/Blueprints/Weapons/BP_BaseWeapon.CurrentRange` _currentweapon))
          (switch `/Game/Blueprints/Enumenators/ENUM_NPCType` (`.Type_11_B5C92BCE436A1CB1F32936A841E63057` (break `/Game/Blueprints/Structure/STRUCT_MainStats` (`/Game/Blueprints/Components/BP_MainStatsComponent.MainStats` (`/Game/Blueprints/Characters/BP_BaseCharacter.BP_MainStatsComponent` (`self.CurrentCharacter`)))))
            (:`NewEnumerator1`
              (set `self.StepOutDistance` (- (`self.ShootDistance`) (select `/Game/Blueprints/Enumenators/ENUM_WeaponRangeType` (`/Game/Blueprints/Weapons/BP_BaseWeapon.CurrentRangeType` (`/Game/Blueprints/Characters/BP_BaseCharacter.CurrentWeapon` (`self.CurrentCharacter`))) :`NewEnumerator0` (/ (`self.ShootDistance`) 2.0) :`NewEnumerator1` (/ (`self.ShootDistance`) 3.0) :`NewEnumerator2` (/ (`self.ShootDistance`) 4.0))) :!label _label))
            (:`NewEnumerator2`
              (goto _label))
            (:`NewEnumerator3`
              (goto _label))
            (:`NewEnumerator4`
              (set `self.StepOutDistance` 0.0))
            (:`NewEnumerator5`
              (goto _label))))
        (:`else`)))
    (:`then_1`
      (bind _output_get (set `PawnSensingComponent.SightRadius` (`.SenseRadius_18_A4EA956649FE5F2E3097F6B8E9962047` (break `/Game/Blueprints/Structure/STRUCT_MainStats` (`/Game/Blueprints/Components/BP_MainStatsComponent.MainStats` (`/Game/Blueprints/Characters/BP_BaseCharacter.BP_MainStatsComponent` (`self.CurrentCharacter`))))) (`/Game/Blueprints/Characters/NPC/BP_BaseNPC.PawnSensing` (`self.CurrentCharacter`))))
      (set `PawnSensingComponent.LOSHearingThreshold` (/ _output_get 2.0) (`/Game/Blueprints/Characters/NPC/BP_BaseNPC.PawnSensing` (`self.CurrentCharacter`))))
    (:`then_2`
      (set `self.CurrentCharacterConfigured` true))))

(fn `UpdateCurrentPlayer`
  (bind _asbp_player_charcter (cast `/Game/Blueprints/Characters/Player/BP_PlayerCharcter` (`GameplayStatics.GetPlayerPawn` 0)))
  (set `self.PlayerCharacter` _asbp_player_charcter)
  (set `self.Destination` (.location (`self.GetTransform` (`self.PlayerCharacter`)))))

(fn `UserConstructionScript`)

(fn `Waiting`
  (`/Game/Blueprints/Characters/BP_BaseCharacter.ActionMain` (`self.CurrentCharacter`) false))

(fn `WaitingOnPatrollPoint`
  (switch `/Game/Blueprints/Enumenators/ENUM_AIStates` (`self.AIState`)
    (:`NewEnumerator0`
      (set `self.AIState` "NewEnumerator1"))))