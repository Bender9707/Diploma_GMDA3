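; Base projectile actor that, on hit, stores the hit data, applies physics and damage, spawns an impact effect, then destroys itself.
; Simulating components get a velocity-scaled impulse, while other valid components trigger its RadialForce.
; Damage and type go to the target's BP_MainStatsComponent, and BP_ImpactEffect attaches to the hit component, normal-aligned with random roll.
; AddDamage increases the damage and prints the new total.
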(event `self.ReceiveHit`
  (params (MyComp :type "PrimitiveComponent Object Reference") (Other :type "Actor Object Reference") (OtherComp :type "PrimitiveComponent Object Reference") (bSelfMoved :type Boolean) (HitLocation :type "Vector Structure") (HitNormal :type "Vector Structure") (NormalImpulse :type "Vector Structure") (Hit :type "HitResult Structure (by ref)"))
  (set `self.OtherActor` Other)
  (set `self.OtherHitComp` OtherComp)
  (set `self.HitLocation` HitLocation)
  (set `self.HitNormal` HitNormal)
  (`|ExecutionSequence`
    (:`then_0`
      (`self.AddPhysicsImpulse `))
    (:`then_1`
      (`self.MakeDamage`))
    (:`then_2`
      (`self.SpawnDecal`))
    (:`then_3`
      (`self.OnEndOfHit`))))

(fn `AddDamage`
  (params (DamageAdd :type Integer))
  (set `self.ProjectileDamage` (+ DamageAdd (`self.ProjectileDamage`)))
  (`KismetSystemLibrary.PrintString` (`KismetStringLibrary.Conv_IntToString` (`self.ProjectileDamage`)) true false))

(fn `AddPhysicsImpulse `
  (bind _otherhitcomp (`self.OtherHitComp`)
    (:`then`
      (if (`SceneComponent.IsSimulatingPhysics` _otherhitcomp "None")
        (`PrimitiveComponent.AddImpulseAtLocation` (`self.OtherHitComp`) (* (`self.GetVelocity`) (`self.ImpulseMult`)) (`self.K2_GetActorLocation`) "None")
        (else
          (`RadialForceComponent.FireImpulse` (`self.RadialForce`)))))
    (:`else`)))

(fn `MakeDamage`
  (bind _otheractor (`self.OtherActor`)
    (:`then`
      (bind _returnvalue (`self.GetComponentByClass` _otheractor "/Game/Blueprints/Components/BP_MainStatsComponent.BP_MainStatsComponent_C"))
      (`/Engine/EditorBlueprintResources/StandardMacros.IsValid` _returnvalue
        (:`Is Valid`
          (`/Game/Blueprints/Components/BP_MainStatsComponent.ReceveDamage` _returnvalue (`self.ProjectileDamage`) (`self.DamageType`)))))
    (:`else`)))

(fn `OnEndOfHit`
  (`self.K2_DestroyActor`))

(fn `SpawnDecal`
  (locals (L_Rot :type "Rotator Structure"))
  (set `local.L_Rot` (`KismetMathLibrary.MakeRotator` (`KismetMathLibrary.RandomFloatInRange` 0.0 360.0) (.pitch (`KismetMathLibrary.Conv_VectorToRotator` (`self.HitNormal`))) (.yaw (`KismetMathLibrary.Conv_VectorToRotator` (`self.HitNormal`)))))
  (bind _returnvalue (`|SpawnActorFromClass` "/Game/Blueprints/Weapons/Projectiles/BP_ImpactEffect.BP_ImpactEffect_C" (`KismetMathLibrary.MakeTransform` (`self.HitLocation`) (`local.L_Rot`)) "Undefined" "OverrideRootScale" null null))
  (`self.K2_AttachToComponent` _returnvalue (`self.OtherHitComp`) "None" "KeepWorld" "KeepWorld" "KeepWorld" true))

(fn `UserConstructionScript`
  (`parent.UserConstructionScript`))