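; Base weapon actor that fires projectiles by weapon type, with magazine, reserve ammo and reloading.
; WeaponConfigure loads stats and mesh from DT_Weapons by ID and scales damage by the owning character's multiplier.
; While active, Tick polls fire input and a state enum, spawning projectile and muzzle FX, with timers for shot and reload delays.
; An event dispatcher broadcasts ammo and state changes, and ActivateWeapon toggles mesh visibility.
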(event `self.ReceiveTick`
  (params (DeltaSeconds :type "Float (single-precision)"))
  (`parent.ReceiveTick` DeltaSeconds)
  (if (`self.IsWeaponActive`)
    (`self.Shooting`)))

(fn `ActivateWeapon`
  (params (Activation :type Boolean))
  (locals (L_Skel :type "Array of SkeletalMeshComponent Object Reference") (L_Stat :type "Array of StaticMeshComponent Object Reference"))
  (set `self.IsWeaponActive` Activation)
  (set `local.L_Skel` (`self.K2_GetComponentsByClass` "/Script/Engine.SkeletalMeshComponent"))
  (set `local.L_Stat` (`self.K2_GetComponentsByClass` "/Script/Engine.StaticMeshComponent"))
  (`|ExecutionSequence`
    (:`then_0`
      (if (> (`KismetArrayLibrary.Array_Length` (`local.L_Skel`)) 0)
        (for _array_element (`local.L_Skel`)
          (`SceneComponent.SetVisibility` _array_element (`self.IsWeaponActive`) true))))
    (:`then_1`
      (if (> (`KismetArrayLibrary.Array_Length` (`local.L_Stat`)) 0)
        (for _array_element_2 (`local.L_Stat`)
          (`SceneComponent.SetVisibility` _array_element_2 (`self.IsWeaponActive`) true))))))

(fn `AfterReloadDelayEnd`
  (set `self.WeaponState` "NewEnumerator0"))

(fn `AfterShotDelayEnd`)

(fn `AmmoUpdate`
  (params (InAmmo :type Integer) (Increased :type Boolean))
  (returns (OutAmmo :type Integer))
  (locals (L_Ammo :type Integer) (L_Current :type Integer))
  (set `local.L_Ammo` InAmmo)
  (if Increased
    (if (> (`self.AmmoCurrent`) 0)
      _
      (elif (not (> (`self.RoundCurrent`) 0))
        (set `self.WeaponState` "NewEnumerator2")))
    (bind _output_get (set `local.L_Current` (+ (`self.AmmoCurrent`) (`local.L_Ammo`))))
    (if (< _output_get (`self.AmmoMax`))
      (set `self.AmmoCurrent` (`local.L_Current`))
      (else
        (set `self.AmmoCurrent` (`self.AmmoMax`))))
    (else
      (bind _output_get_2 (set `local.L_Current` (- (`self.AmmoCurrent`) (`local.L_Ammo`))))
      (if (> _output_get_2 0)
        (set `self.AmmoCurrent` (`local.L_Current`))
        (else
          (set `self.AmmoCurrent` 0)
          (`self.OnWeaponStatusChanged`)
          (return (+ (`self.RoundMax`) (`local.L_Current`)))))))
  (`self.OnWeaponStatusChanged`)
  (return (`self.RoundMax`)))

(fn `Reload`
  (set `self.WeaponState` "NewEnumerator3")
  (`AudioComponent.Play` (`self.ReloadStartSound`) 0.0)
  (bind _outammo (`self.AmmoUpdate` (- (`self.RoundMax`) (`self.RoundCurrent`))))
  (bind _output_get (set `self.RoundCurrent` _outammo))
  (if (!= _output_get 0)
    (`KismetSystemLibrary.K2_SetTimerDelegate` (`|CreateDelegate` :!event `AfterReloadDelayEnd`) (`self.CurrentReloadTime`))
    (else
      (set `self.WeaponState` "NewEnumerator4")
      (`self.OnWeaponStatusChanged`))))

(fn `RoundsCount`
  (returns (AllowShooting :type Boolean))
  (bind _result (`/Engine/EditorBlueprintResources/StandardMacros.DecrementInt` (`self.RoundCurrent`))
    (:`  `
      (return (> _result 0)))))

(fn `Shooting`
  (if (and (`self.InProcess`) (`|EnumEquality` (`self.WeaponState`) "NewEnumerator0"))
    (`self.SingleShot`)
    (bind _allowshooting (`self.RoundsCount`))
    (if _allowshooting
      (`KismetSystemLibrary.K2_SetTimerDelegate` (`|CreateDelegate` :!event `AfterReloadDelayEnd`) (`self.AfterShotDelay`))
      (set `self.WeaponState` "NewEnumerator1")
      (`self.OnWeaponStatusChanged`)
      (else
        (set `self.WeaponState` "NewEnumerator2")
        (if (`self.IsAutoReloading`)
          (`self.Reload`)
          (else
            (`self.OnWeaponStatusChanged`)))))))

(fn `ShootInputRecived`
  (params (InProcess :type Boolean))
  (set `self.InProcess` InProcess))

(fn `SingleShot`
  (bind _returnvalue (`|SpawnActorFromClass` (select `/Game/Blueprints/Enumenators/ENUM_WeaponType` (`self.CurrenWeaponType`) :`NewEnumerator0` "/Game/Blueprints/Weapons/Projectiles/BP_BaseProjectile_PistolBullet.BP_BaseProjectile_PistolBullet_C" :`NewEnumerator1` "/Game/Blueprints/Weapons/Projectiles/BP_BaseProjectile_RifleBullet.BP_BaseProjectile_RifleBullet_C" :`NewEnumerator2` "/Game/Blueprints/Weapons/Projectiles/BP_BaseProjectile_ShotgunBullet.BP_BaseProjectile_ShotgunBullet_C" :`NewEnumerator3` "/Game/Blueprints/Weapons/Projectiles/BP_BaseProjectile_Rocket.BP_BaseProjectile_Rocket_C" :!type "Actor Class Reference") (`SceneComponent.K2_GetComponentToWorld` (`self.Muzzle`)) "Undefined" "OverrideRootScale" null null))
  (cast `/Game/Blueprints/Weapons/Projectiles/BP_BaseProjectile` _returnvalue)
  (`AudioComponent.Play` (`self.ShotS`) 0.0)
  (bind _returnvalue_2 (`|SpawnActorFromClass` "/Game/Blueprints/Weapons/Projectiles/BP_MuzzleFX.BP_MuzzleFX_C" (`SceneComponent.K2_GetComponentToWorld` (`self.Muzzle`)) "Undefined" "OverrideRootScale" null null))
  (`self.K2_AttachToComponent` _returnvalue_2 (`self.Muzzle`) "None" "SnapToTarget" "SnapToTarget" "SnapToTarget" true))

(fn `UserConstructionScript`
  (`parent.UserConstructionScript`))

(fn `WeaponConfigure`
  (params (InWeaponID :type Name))
  (returns (Success :type Boolean))
  (bind (_weapontype _nickname _rounds _roundsinpocket _damage _shottime _reloadtime _autoreload _rangetipe _range) (break `/Game/Blueprints/Structure/STRUCT_WeaponStats` (`self.WeaponStats`)))
  (bind ((`Mesh_31_450772F54BC15900A2B88BA87DD8CC82` _mesh)) (break `/Game/Blueprints/Structure/STRUCT_WeaponStats` (`self.WeaponStats`)))
  (set `self.WeaponID` InWeaponID)
  (bind _returnvalue (`|GetDataTableRow` "/Game/Data_Table/DT_Weapons.DT_Weapons" (`self.WeaponID`))
    (:`then`
      (set `self.WeaponStats` _returnvalue)
      (set `self.CurrenWeaponType` _weapontype)
      (set `self.RoundMax` _rounds)
      (set `self.RoundCurrent` _rounds)
      (set `self.CurrentDamage` _damage)
      (set `self.AfterShotDelay` _shottime)
      (set `self.IsAutoReloading` _autoreload)
      (set `self.CurrentRangeType` _rangetipe)
      (set `self.CurrentRange` _range)
      (set `self.AmmoMax` (`.RoundsInPocket_11_C82E700842C3D3B379E64D88BC29CF59` (break `/Game/Blueprints/Structure/STRUCT_WeaponStats` (`self.WeaponStats`))))
      (set `self.AmmoCurrent` (`self.RoundMax`))
      (if (`KismetSystemLibrary.IsValid` _mesh)
        (`StaticMeshComponent.SetStaticMesh` (`self.StaticMeshWeapon`) _mesh))
      (bind _asbp_base_character (cast `/Game/Blueprints/Characters/BP_BaseCharacter` (`self.GetOwner`))
        (:`then`
          (set `self.CurrentDamage` (`KismetMathLibrary.FTrunc` (* (`self.CurrentDamage`) (`.DamageMuit_15_B7CF996D486B3FCEA7BB22BFB3CA2A0A` (break `/Game/Blueprints/Structure/STRUCT_MainStats` (`/Game/Blueprints/Components/BP_MainStatsComponent.MainStats` (`/Game/Blueprints/Characters/BP_BaseCharacter.BP_MainStatsComponent` _asbp_base_character)))))))
          (set `self.Nickname` (`.Nickname_9_789096DD4B27956EF05B6D95F1A916AD` (break `/Game/Blueprints/Structure/STRUCT_WeaponStats` (`self.WeaponStats`))))
          (return true))
        (:`CastFailed`
          (`KismetSystemLibrary.PrintString` "Something Wrong With Statick Mesh :(" true true (struct :`R` 1.0 :`B` 0.97267 :`A` 1.0) 10.0)
          (return false))))
    (:`RowNotFound`
      (`KismetSystemLibrary.PrintString` "Spow Weapon Not Success :(" true true (struct :`R` 1.0 :`B` 0.97267 :`A` 1.0) 10.0)
      (return false))))