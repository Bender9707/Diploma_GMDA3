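; Trap trigger that damages actors with a BP_MainStatsComponent in contact with its Box.
; BeginPlay overlap checks and begin overlap store a single damage receiver and set a DOT timer, which has zero time and no looping, so no repeating damage is scheduled.
; DOTEvent damages the stored receiver.
; End overlap deals damage to the leaving actor, then clears the receiver and any valid timer.
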(event `self.ReceiveBeginPlay`
  (`parent.ReceiveBeginPlay`)
  (for _array_element (`PrimitiveComponent.GetOverlappingActors` (`self.Box`) "/Script/Engine.Actor")
    (bind _returnvalue (`self.GetComponentByClass` _array_element "/Game/Blueprints/Components/BP_MainStatsComponent.BP_MainStatsComponent_C"))
    (`/Engine/EditorBlueprintResources/StandardMacros.IsValid` _returnvalue
      (:`Is Valid`
        (set `self.DamageReceiverComp` _returnvalue)
        (if (not (`KismetSystemLibrary.K2_IsValidTimerHandle` (`self.DOTTimerHandler`)))
          (bind _returnvalue_2 (`KismetSystemLibrary.K2_SetTimerDelegate` (delegate `DOTEvent`) :!label _label))
          (set `self.DOTTimerHandler` _returnvalue_2))))))

(event `self.Box.OnComponentBeginOverlap`
  (params (OverlappedComponent :type "PrimitiveComponent Object Reference") (OtherActor :type "Actor Object Reference") (OtherComp :type "PrimitiveComponent Object Reference") (OtherBodyIndex :type Integer) (bFromSweep :type Boolean) (SweepResult :type "HitResult Structure (by ref)"))
  (bind _returnvalue (`self.GetComponentByClass` OtherActor "/Game/Blueprints/Components/BP_MainStatsComponent.BP_MainStatsComponent_C"))
  (`/Engine/EditorBlueprintResources/StandardMacros.IsValid` _returnvalue
    (:`Is Valid`
      (set `self.DamageReceiverComp` _returnvalue)
      (goto _label))))

(event `DOTEvent`
  (bind _damagereceivercomp (`self.DamageReceiverComp`)
    (:`then`
      (`/Game/Blueprints/Components/BP_MainStatsComponent.ReceveDamage` _damagereceivercomp (`self.Damage`) (`self.DamageType`)))
    (:`else`)))

(event `self.Box.OnComponentEndOverlap`
  (params (OverlappedComponent :type "PrimitiveComponent Object Reference") (OtherActor :type "Actor Object Reference") (OtherComp :type "PrimitiveComponent Object Reference") (OtherBodyIndex :type Integer))
  (bind _returnvalue (`self.GetComponentByClass` OtherActor "/Game/Blueprints/Components/BP_MainStatsComponent.BP_MainStatsComponent_C"))
  (`/Engine/EditorBlueprintResources/StandardMacros.IsValid` _returnvalue
    (:`Is Valid`
      (`/Game/Blueprints/Components/BP_MainStatsComponent.ReceveDamage` _returnvalue (`self.Damage`) (`self.DamageType`))
      (set `self.DamageReceiverComp` null)
      (if (`KismetSystemLibrary.K2_IsValidTimerHandle` (`self.DOTTimerHandler`))
        (`KismetSystemLibrary.K2_ClearAndInvalidateTimerHandle` (`self.DOTTimerHandler`))))))

(fn `UserConstructionScript`
  (`parent.UserConstructionScript`))