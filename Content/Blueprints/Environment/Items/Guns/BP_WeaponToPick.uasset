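; Weapon pickup actor that spins in the world from a random starting yaw, turning by RotationSpeed every tick.
; When the player character overlaps its sphere while the current weapon is ready to shoot or empty, it grants the weapon set by WeaponByID.
; An already owned weapon gets RoundMax ammo added; a new one joins the available list and is configured on the player.
; The pickup destroys itself once used.
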(event `self.ReceiveBeginPlay`
  (`parent.ReceiveBeginPlay`)
  (`SceneComponent.K2_AddRelativeRotation` (`self.StaticMesh`) (`KismetMathLibrary.MakeRotator` 0.0 0.0 (`KismetMathLibrary.RandomFloatInRange` 0.0 360.0)) false false))

(event `self.ReceiveTick`
  (params (DeltaSeconds :type "Float (single-precision)"))
  (`parent.ReceiveTick` DeltaSeconds)
  (`SceneComponent.K2_AddRelativeRotation` (`self.StaticMesh`) (`KismetMathLibrary.MakeRotator` 0.0 0.0 (`self.RotationSpeed`)) false false))

(event `self.Sphere.OnComponentBeginOverlap`
  (params (OverlappedComponent :type "PrimitiveComponent Object Reference") (OtherActor :type "Actor Object Reference") (OtherComp :type "PrimitiveComponent Object Reference") (OtherBodyIndex :type Integer) (bFromSweep :type Boolean) (SweepResult :type "HitResult Structure (by ref)"))
  (bind _asbp_player_charcter (cast `/Game/Blueprints/Characters/Player/BP_PlayerCharcter` OtherActor))
  (set `self.PlayerCharacter` _asbp_player_charcter)
  (switch `/Game/Blueprints/Enumenators/ENUM_WeaponState` (`/Game/Blueprints/Weapons/BP_BaseWeapon.WeaponState` (`/Game/Blueprints/Characters/BP_BaseCharacter.CurrentWeapon` (`self.PlayerCharacter`)))
    (:`NewEnumerator0`
      _)
    (:`NewEnumerator4`
      _))
  (`|ExecutionSequence`
    (:`then_0`
      (`self.AddWeaponToPlayer`))
    (:`then_1`
      (if (`self.IsUse`)
        (`self.K2_DestroyActor`)))))

(fn `AddWeaponToPlayer`
  (locals (L_Weap :type "/Game/Blueprints/Weapons/BP_BaseWeapon Object Reference"))
  (bind (_value _returnvalue) (`BlueprintMapLibrary.Map_Find` (`/Game/Blueprints/Characters/BP_BaseCharacter.MapOfWeapon` (`self.PlayerCharacter`)) (`self.WeaponByID`)))
  (if (!= (`self.WeaponByID`) "None")
    (if _returnvalue
      (bind _output_get (set `local.L_Weap` _value))
      (`/Game/Blueprints/Weapons/BP_BaseWeapon.AmmoUpdate` (`local.L_Weap`) (`/Game/Blueprints/Weapons/BP_BaseWeapon.RoundMax` _output_get) true)
      (set `self.IsUse` true)
      (else
        (bind _returnvalue_2 (`KismetArrayLibrary.Array_AddUnique` (`/Game/Blueprints/Characters/BP_BaseCharacter.AvalableWeapon` (`self.PlayerCharacter`)) (`self.WeaponByID`)))
        (`/Game/Blueprints/Characters/BP_BaseCharacter.ConfigureWeapons` (`self.PlayerCharacter`) _returnvalue_2)
        (set `self.IsUse` true)))))

(fn `UserConstructionScript`
  (`parent.UserConstructionScript`))