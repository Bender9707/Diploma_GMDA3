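; BP_Spawner is an environment actor that spawns a limited number of NPCs of a configurable class at its SpawnPoint, optionally starting on BeginPlay.
; SpawnOneNPC stores each new BP_BaseNPC, counts it, and sets a one-shot delay timer, apparently to chain the next spawn, while printing the delay.
; Reaching the count or calling StopSpawnNPCs sets IsDone to block further spawns.
; The patrol-state update is an empty, unconnected stub.
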(event `self.ReceiveBeginPlay`
  (`parent.ReceiveBeginPlay`)
  (if (`self.SpawnOnStart`)
    (`self.StartSpawnNPCs`)))

(fn `SpawnOneNPC`
  (if (not (`self.IsDone`))
    (if (`KismetSystemLibrary.IsValidClass` (`self.SpawnNPCClass`))
      (if (< (`self.Counter`) (`self.NPCsCont`))
        (bind _returnvalue (`|SpawnActorFromClass` (`self.SpawnNPCClass`) (`SceneComponent.K2_GetComponentToWorld` (`self.SpawnPoint`)) "AdjustIfPossibleButAlwaysSpawn" "OverrideRootScale" null null))
        (bind _asbp_base_npc (cast `/Game/Blueprints/Characters/NPC/BP_BaseNPC` _returnvalue))
        (set `self.LastSpawnedNPC` _asbp_base_npc)
        (`/Engine/EditorBlueprintResources/StandardMacros.IncrementInt` (`self.Counter`)
          (:`  `
            (`KismetSystemLibrary.K2_SetTimerDelegate` (`|CreateDelegate` :!event `SpawnOneNPC`) (`self.BetweenSpawnDelay`))
            (`KismetSystemLibrary.PrintString` (`KismetStringLibrary.Conv_DoubleToString` (`self.BetweenSpawnDelay`)) true false)))
        (else
          (set `self.IsDone` true))))))

(fn `StartSpawnNPCs`
  (`self.SpawnOneNPC`))

(fn `StopSpawnNPCs`
  (set `self.IsDone` true))

(fn `UpdatePatrolStateForSpawnedNPC`)

(fn `UserConstructionScript`
  (`parent.UserConstructionScript`))