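; AI helper actor in the environment spawner set that tracks whether its spot is free of NPCs through a Vacant flag.
; On BeginPlay it clears Vacant if its Sphere already overlaps a BP_BaseNPC.
; Sphere overlap events then clear the flag when an NPC enters and set it when one leaves, without checking whether other NPCs remain inside.
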(event `self.ReceiveBeginPlay`
  (`parent.ReceiveBeginPlay`)
  (if (`KismetArrayLibrary.Array_IsValidIndex` (`PrimitiveComponent.GetOverlappingActors` (`self.Sphere`) "/Game/Blueprints/Characters/NPC/BP_BaseNPC.BP_BaseNPC_C"))
    (set `self.Vacant` false)))

(event `self.Sphere.OnComponentBeginOverlap`
  (params (OverlappedComponent :type "PrimitiveComponent Object Reference") (OtherActor :type "Actor Object Reference") (OtherComp :type "PrimitiveComponent Object Reference") (OtherBodyIndex :type Integer) (bFromSweep :type Boolean) (SweepResult :type "HitResult Structure (by ref)"))
  (cast `/Game/Blueprints/Characters/NPC/BP_BaseNPC` OtherActor)
  (set `self.Vacant` false))

(event `self.Sphere.OnComponentEndOverlap`
  (params (OverlappedComponent :type "PrimitiveComponent Object Reference") (OtherActor :type "Actor Object Reference") (OtherComp :type "PrimitiveComponent Object Reference") (OtherBodyIndex :type Integer))
  (cast `/Game/Blueprints/Characters/NPC/BP_BaseNPC` OtherActor)
  (set `self.Vacant` true))

(fn `UserConstructionScript`
  (`parent.UserConstructionScript`))